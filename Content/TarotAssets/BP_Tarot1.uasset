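; Tarot card actor that takes its face U and V values from an NPC reference.
; The construction script creates a dynamic material instance from the static mesh's first material and stores it as DIMTarotFace, without assigning it to the mesh.
; BeginPlay copies U and V from the NPC, but the nodes that set those material parameters are unconnected, so the values never reach the material.
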(event EventBeginPlay
  (bind _npc (Variables|Default|GetNPC))
  (Variables|Default|SetU (Variables|/Game/MetaHumans/lexa/BP_lexa.BP_lexa_C|GetU _npc))
  (Variables|Default|SetV (Variables|/Game/MetaHumans/lexa/BP_lexa.BP_lexa_C|GetV _npc)))

(event Collision|EventActorBeginOverlap
  (params (OtherActor :type Actor%20Object%20Reference)))

(event EventTick
  (params (DeltaSeconds :type Float%20%28single-precision%29)))

(fn ConstructionScript
  (bind _returnvalue (Rendering|Material|CreateDynamicMaterialInstance (Rendering|Material|GetMaterial (Variables|Default|GetStaticMesh) 0) "Face" "None" :!class /Script/Engine.KismetMaterialLibrary))
  (Variables|Default|SetDIM_TarotFace _returnvalue))